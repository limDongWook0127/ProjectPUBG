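; Player character Blueprint for what appears to be a battle-royale game, covering airplane-drop parachuting, swimming and punching.
; BeginPlay spawns a hidden socketed parachute and hand punch capsules; Tick detects the high-altitude drop, enabling low gravity, banked steering and camera zoom until landing.
; Left-punch overlaps send GAS hit events; the construction script links equipment meshes via leader pose.
; Recoil timeline and inventory debug keys are included.
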(event `TESTRECoil`
  (params (Min :type "Float (double-precision)") (Max :type "Float (double-precision)") (MaxY :type "Float (double-precision)"))
  ;[1 1 1] 코멘트
  (bind (_direction `_새_트랙_0`) (`Timeline|타임라인` :!via `PlayFromStart`)
    (:`Update`
      (`self.AddControllerPitchInput` (* `_새_트랙_0` MaxY))
      (`self.AddControllerYawInput` (* `_새_트랙_0` (`KismetMathLibrary.RandomFloatInRange` Min Max))))))

(event `self.ReceiveBeginPlay`
  (bind _mesh (`self.Mesh`))
  (`|ExecutionSequence`
    (:`then_0`
      (set `self.MapZ` (+ (.z (`.Max` (break `Box` (`BaseGameState.LandScapeBoundingBox` (cast `BaseGameState` (`GameplayStatics.GetGameState`) :!pure true))))) 5000.0)))
    (:`then_1`
      (bind _returnvalue (`|SpawnActorFromClass` "/Game/Blueprint/GameplayActor/Parachute/BP_Parachute.BP_Parachute_C" (`SceneComponent.GetSocketTransform` (`self.Mesh`) "Parachute" "RTS_World") "Undefined" "MultiplyWithRoot" self self))
      (bind _output_get (set `self.Parachute` _returnvalue))
      (`self.SetOwner` _output_get self)
      (`self.SetActorHiddenInGame` _output_get true)
      (`SceneComponent.K2_AttachToComponent` (`Actor.RootComponent` _output_get) (`self.Mesh`) "Parachute" "SnapToTarget" "SnapToTarget" "KeepRelative" true))
    (:`then_2`
      (`SceneComponent.K2_AttachToComponent` (`self.PunchCapsuleRight`) _mesh "hand_r" "SnapToTarget" "SnapToTarget" "KeepRelative" true)
      (`SceneComponent.K2_AttachToComponent` (`self.PunchCapsuleLeft`) _mesh "hand_l" "SnapToTarget" "SnapToTarget" "KeepRelative" true))))

(event `Parachute Zoom Out`
  (`self.ModifyGravity` 1.0)
  (set `CharacterMovementComponent.AirControl` 0.0 (`self.CharacterMovement`)))

(event `ParachuteZoomIn`
  (bind _charactermovement (`self.CharacterMovement`))
  (`self.ModifyGravity` 0.1)
  (set `CharacterMovementComponent.AirControl` 200.0 _charactermovement)
  (set `MovementComponent.Velocity` (`KismetMathLibrary.MakeVector` (.x (`self.GetVelocity`)) (.y (`self.GetVelocity`)) -300.0) _charactermovement))

(event `Start Swimming`
  (set `self.IsSwimming` true)
  (`PUBGSpringArmComponent.BP_TimelineAddOffset` (`self.CameraBoom`) (0.0 0.0 -40.0) 0.2))

(event `CLZoomOut`
  (bind (_direction `_새_트랙_0`) (`Timeline|타임라인_1` :!via `ReverseFromEnd`)
    (:`Update`
      (set `SpringArmComponent.TargetArmLength` `_새_트랙_0` (`self.CameraBoom`)))))

(event `CLZoomin`
  (bind (_direction `_새_트랙_0`) (`Timeline|타임라인_0` :!via `PlayFromStart`)
    (:`Update`
      (set `SpringArmComponent.TargetArmLength` `_새_트랙_0` (`self.CameraBoom`)))))

(event `Stop Swimming`
  (set `self.IsSwimming` false)
  (`PUBGSpringArmComponent.BP_TimelineAddOffset` (`self.CameraBoom`) (0.0 0.0 40.0) 0.2))

(event `Server_Destroy`
  (`self.K2_DestroyActor` (`self.Parachute`)))

(event `self.OnLanded`
  (params (Hit :type "HitResult Structure (by ref)"))
  (if (`self.OnTheFirstAirPlane`)
    (`/Engine/EditorBlueprintResources/StandardMacros.DoOnce` false
      (:`Completed`
        (`self.SetOntheParachute_Server` false)
        (`self.Parachute Zoom Out`)
        (`self.CLZoomOut`)
        (`self.Server_Destroy`)))))

(event `self.ReceiveTick`
  (params (DeltaSeconds :type "Float (single-precision)"))
  (bind (_returnvalue_x _returnvalue_y _returnvalue_z) (`KismetMathLibrary.BreakVector` (`self.K2_GetActorLocation`)))
  (`|ExecutionSequence`
    (:`then_0`
      (if (> _returnvalue_z (`self.MapZ`))
        (set `self.OnTheFirstAirPlane` true)))
    (:`then_1`
      (if (and (`self.OnTheFirstAirPlane`) (`self.OntheParachute`))
        (`/Engine/EditorBlueprintResources/StandardMacros.DoOnce` false
          (:`Completed`
            (`self.SetOntheParachute_Server` true)
            (`self.ParachuteZoomIn`)
            (`self.CLZoomin`)))))))

(event `SetOntheParachute_Server`
  (params (NewParam :type Boolean :default true))
  (`self.SetOntheParachute` NewParam))

(event `Key|Tab`
  (params (Key :type "Key Structure")))

(event `Key|F`
  (params (Key :type "Key Structure")))

(event `self.Input_Move`
  (params (InputActionValue :type "InputActionValue Structure (by ref)"))
  (bind (_returnvalue_roll _returnvalue_pitch _returnvalue_yaw) (`KismetMathLibrary.BreakRotator` (`self.K2_GetActorRotation`)))
  (bind (_returnvalue_roll_2 _returnvalue_pitch_2 _returnvalue_yaw_2) (`KismetMathLibrary.BreakRotator` (`self.K2_GetActorRotation`)))
  (bind (_returnvalue_roll_3 _returnvalue_pitch_3 _returnvalue_yaw_3) (`KismetMathLibrary.BreakRotator` (`self.K2_GetActorRotation`)))
  (bind (_returnvalue_roll_4 _returnvalue_pitch_4 _returnvalue_yaw_4) (`KismetMathLibrary.BreakRotator` (`self.K2_GetActorRotation`)))
  (bind (_returnvalue_roll_5 _returnvalue_pitch_5 _returnvalue_yaw_5) (`KismetMathLibrary.BreakRotator` (`self.K2_GetActorRotation`)))
  (`|ExecutionSequence`
    (:`then_0`
      (if (`self.OntheParachute`)
        (if (< InputActionValue_X 0.0)
          (`|ExecutionSequence`
            (:`then_0`
              (if (not (< (`self.ActorRotate`) -30.0))
                (bind _output_get (set `self.ActorRotate` _returnvalue_roll_4))
                (bind _returnvalue (`KismetMathLibrary.MakeRotator` (- _output_get 1.0) _returnvalue_pitch_4 _returnvalue_yaw_4))
                (`self.K2_SetActorRotation` _returnvalue)
                (set `self.RotateVector` (`KismetMathLibrary.Conv_RotatorToVector` _returnvalue))))
            (:`then_1`
              (`self.K2_SetActorRotation` (`KismetMathLibrary.MakeRotator` _returnvalue_roll_5 _returnvalue_pitch_5 (- _returnvalue_yaw_5 (`self.RotateSpeed`))))
              (if (not (< (`KismetMathLibrary.Abs` (`self.ActorRotate`)) 1.0))
                (bind (_direction `_새_트랙_0`) (`Timeline|Timeline` :!via `PlayFromStart` :!label _label)
                  (:`Update`
                    (`self.K2_SetActorRotation` (`KismetMathLibrary.MakeRotator` (* `_새_트랙_0` _returnvalue_roll_2) _returnvalue_pitch_2 _returnvalue_yaw_2)))
                  (:`Finished`
                    (set `self.ActorRotate` 0.0))))))
          (elif (> InputActionValue_X 0.0)
            (`|ExecutionSequence`
              (:`then_0`
                (if (not (> (`self.ActorRotate`) 30.0))
                  (bind _output_get_2 (set `self.ActorRotate` _returnvalue_roll_3))
                  (`self.K2_SetActorRotation` (`KismetMathLibrary.MakeRotator` (+ _output_get_2 1.0) _returnvalue_pitch_3 _returnvalue_yaw_3))))
              (:`then_1`
                (`self.K2_SetActorRotation` (`KismetMathLibrary.MakeRotator` _returnvalue_roll _returnvalue_pitch (+ _returnvalue_yaw (`self.RotateSpeed`))))
                (if (not (< (`KismetMathLibrary.Abs` (`self.ActorRotate`)) 1.0))
                  (goto _label :!via `PlayFromStart`))))))))
    (:`then_1`
      (if (`self.OntheParachute`)
        (if (not (< InputActionValue_Y 1.0))
          (`self.AddMovementInput` (`KismetMathLibrary.Conv_RotatorToVector` (`self.K2_GetActorRotation`)) (* InputActionValue_Y 0.8)))))))

(event `Key|NumPadOne`
  (params (Key :type "Key Structure"))
  (bind _inventorycomponent (`self.InventoryComponent`))
  (:`Pressed`
    (`InventoryComponent.PrintContents` _inventorycomponent)
    (`InventoryComponent.ServerPrintContents` _inventorycomponent)))

(event `Key|NumPadTwo`
  (params (Key :type "Key Structure"))
  (bind _nearcomponent (`self.NearComponent`))
  (:`Pressed`
    (`NearComponent.PrintGroundItems` _nearcomponent)
    (`NearComponent.ServerPrintGroundItems` _nearcomponent)))

(event `Key|NumPadThree`
  (params (Key :type "Key Structure"))
  (bind _equippedcomponent (`self.EquippedComponent`))
  (:`Pressed`
    (`EquippedComponent.PrintEquippedItems` _equippedcomponent)
    (`EquippedComponent.ServerPrintEquippedItems` _equippedcomponent)))

(event `self.PunchCapsuleRight.OnComponentBeginOverlap`
  (params (OverlappedComponent :type "PrimitiveComponent Object Reference") (OtherActor :type "Actor Object Reference") (OtherComp :type "PrimitiveComponent Object Reference") (OtherBodyIndex :type Integer) (bFromSweep :type Boolean) (SweepResult :type "HitResult Structure (by ref)")))

(event `self.PunchCapsuleLeft.OnComponentBeginOverlap`
  (params (OverlappedComponent :type "PrimitiveComponent Object Reference") (OtherActor :type "Actor Object Reference") (OtherComp :type "PrimitiveComponent Object Reference") (OtherBodyIndex :type Integer) (bFromSweep :type Boolean) (SweepResult :type "HitResult Structure (by ref)"))
  (`KismetSystemLibrary.PrintString` (`KismetSystemLibrary.GetDisplayName` OtherActor))
  (if (not (== self OtherActor))
    (`AbilitySystemBlueprintLibrary.SendGameplayEventToActor` OtherActor (struct :`TagName` "Player.Event.Action.Hit") (make `GameplayEventData` (struct) self OtherActor null null (struct) (struct) (struct) 20.0))))

(fn `UserConstructionScript`
  (`|ExecutionSequence`
    (:`then_0`
      (bind _enumvalue (foreach `EPlayerMeshType` false)
        (:`LoopBody`
          (`SkinnedMeshComponent.SetLeaderPoseComponent` (`BlueprintMapLibrary.Map_Find` (`self.CharacterEquipmentMap`) _enumvalue) (`self.Mesh`) false false))))
    (:`then_1`
      (set `self.Location` (`SceneComponent.GetSocketLocation` (`self.Mesh`) "item_rSocket")))))