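; Gameplay ability that leans the player character to the left.
; On activation, unless a prone request is set or the character is falling, it moves the camera, starts leaning on PlayerMovementComponent and adds the InputTag.LeftLeaning tag.
; On end, it restores the camera, stops leaning and removes the tag, but only under the same guard, read from the component reference cached at activation.
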(event `self.K2_ActivateAbility`
  (bind _returnvalue (`self.GetPlayerCharacterFromActorInfo`))
  (bind _asplayer_movement_component (cast `PlayerMovementComponent` (`Character.CharacterMovement` (`self.GetPlayerCharacterFromActorInfo`))))
  (if (and (not (`PlayerMovementComponent.RequestToStartProne` _asplayer_movement_component)) (not (`NavMovementComponent.IsFalling` _asplayer_movement_component)))
    (`PlayerCharacter.LeftLeanCameraMovement` _returnvalue)
    (`PlayerMovementComponent.StartLeaning` _asplayer_movement_component -1.0)
    (`BaseFunctionLibrary.AddGameplayTagToActor` _returnvalue (struct :`TagName` "InputTag.LeftLeaning"))))

(event `self.K2_OnEndAbility`
  (params (bWasCancelled :type Boolean))
  (bind _returnvalue (`self.GetPlayerCharacterFromActorInfo`))
  (if (and (not (`PlayerMovementComponent.RequestToStartProne` (stale `self.K2_ActivateAbility` _asplayer_movement_component))) (not (`NavMovementComponent.IsFalling` (stale `self.K2_ActivateAbility` _asplayer_movement_component))))
    (bind _asplayer_movement_component (cast `PlayerMovementComponent` (`Character.CharacterMovement` _returnvalue)))
    (`PlayerCharacter.LeftDefaultCameraMovement` _returnvalue)
    (`PlayerMovementComponent.StopLeaning` _asplayer_movement_component)
    (`BaseFunctionLibrary.RemoveGameplayTagFromActor` _returnvalue (struct :`TagName` "InputTag.LeftLeaning"))))