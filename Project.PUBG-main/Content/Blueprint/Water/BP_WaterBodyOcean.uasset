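; Ocean water body Blueprint that switches the player character into and out of swimming on actor overlap.
; On begin overlap it caches the BP_PlayerCharacter, starts swimming and disarms its weapon; end overlap stops swimming but keeps the reference.
; Tick prints the cached character's mesh location as debug output.
; Swimming and floating checks and a water surface depth query are left unconnected.
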(event `self.ReceiveActorBeginOverlap`
  (params (OtherActor :type "Actor Object Reference"))
  (bind _asbp_player_character (cast `/Game/Blueprint/Character/BP_PlayerCharacter` OtherActor))
  (bind _output_get (set `self.As BP Player Character` _asbp_player_character))
  (`/Game/Blueprint/Character/BP_PlayerCharacter.Start Swimming` _output_get)
  (`PlayerCharacter.WeaponDisarmament` _asbp_player_character))

(event `self.ReceiveActorEndOverlap`
  (params (OtherActor :type "Actor Object Reference"))
  (bind _asbp_player_character (cast `/Game/Blueprint/Character/BP_PlayerCharacter` OtherActor))
  (`/Game/Blueprint/Character/BP_PlayerCharacter.Stop Swimming` _asbp_player_character))

(event `self.ReceiveTick`
  (params (DeltaSeconds :type "Float (single-precision)"))
  (`|ExecutionSequence`
    (:`then_0`
      (bind _as_bp_player_character (`self.As BP Player Character`)
        (:`then`
          (`KismetSystemLibrary.PrintString` (`KismetStringLibrary.Conv_VectorToString` (`SceneComponent.K2_GetComponentLocation` (`Character.Mesh` _as_bp_player_character)))))
        (:`else`)))))

(fn `UserConstructionScript`)