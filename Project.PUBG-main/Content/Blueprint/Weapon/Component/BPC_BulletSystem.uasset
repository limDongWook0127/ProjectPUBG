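; Actor component that drives ballistic bullet flight and hit reporting for its owning BP_Test_Projectile.
; On BeginPlay it sets initial velocity from the projectile's direction and speed, then destroys the owner after a lifetime.
; Each server tick line-traces the next step with debug drawing, then either sends a GAS hit event carrying damage and destroys the projectile, or moves it and updates velocity with gravity and quadratic air drag.
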(event `self.ReceiveBeginPlay`
  (bind _asbp_test_projectile (cast `/Game/Blueprint/Weapon/Projectile/BP_Test_Projectile` (`self.GetOwner`)))
  (set `self.As BP Test Projectile` _asbp_test_projectile)
  (`self.ShootBullet`)
  (`KismetSystemLibrary.PrintString` "shoot"))

(event `ShootBullet`
  (set `self.Bullet_Velocity` (* (`/Game/Blueprint/Weapon/Projectile/BP_Test_Projectile.VelocityVector` (`self.As BP Test Projectile`)) (`/Game/Blueprint/Weapon/Projectile/BP_Test_Projectile.BulletSpeed` (`self.As BP Test Projectile`))))
  (set `self.Start_Location` (`Actor.K2_GetActorLocation` (`self.GetOwner`)))
  (set `self.IsBulletInitialized` true)
  (`KismetSystemLibrary.Delay` (`self.BulletLifeTime`))
  (`Actor.K2_DestroyActor` (`self.GetOwner`)))

(event `self.ReceiveTick`
  (params (DeltaSeconds :type "Float (single-precision)"))
  (bind _as_bp_test_projectile (`self.As BP Test Projectile`))
  (`/Engine/EditorBlueprintResources/ActorComponentMacros.Switch Has Authority`
    (:`Authority`
      (if (`self.IsBulletInitialized`)
        (set `self.Delta Seconds` DeltaSeconds)
        (set `self.Start_Location` (`Actor.K2_GetActorLocation` (`self.GetOwner`)))
        (set `self.End_Location` (+ (`self.Start_Location`) (* (`self.Bullet_Velocity`) (`self.Delta Seconds`))))
        (bind (_outhit _returnvalue) (`KismetSystemLibrary.LineTraceSingle` (`self.Start_Location`) (`self.End_Location`) "TraceTypeQuery4" false (`|MakeArray` (`self.IgnoreToActor`)) "ForDuration" true (struct :`R` 1.0 :`A` 1.0) (struct :`G` 1.0 :`A` 1.0) 0.05))
        (if _returnvalue
          (bind (_bblockinghit _binitialoverlap _time _distance _location _impactpoint _normal _impactnormal _physmat _hitactor) (`GameplayStatics.BreakHitResult` _outhit))
          (`AbilitySystemBlueprintLibrary.SendGameplayEventToActor` _hitactor (struct :`TagName` "Player.Event.Action.Hit") (make `GameplayEventData` (struct) (`/Game/Blueprint/Weapon/Projectile/BP_Test_Projectile.Attack_Player` _as_bp_test_projectile) _hitactor null null (struct) (struct) (struct) (`/Game/Blueprint/Weapon/Projectile/BP_Test_Projectile.BulletDamage` _as_bp_test_projectile)))
          (`Actor.K2_DestroyActor` (`self.GetOwner`))
          (else
            (`Actor.K2_SetActorLocation` (`self.GetOwner`) (`self.End_Location`) false false)
            (set `self.Bullet_Velocity` (`self.CalculateGravity` (`self.Bullet_Velocity`)))))))))

(fn `CalculateGravity`
  (params (Velocity :type "Vector Structure"))
  (returns (Return :type "Vector Structure"))
  (bind _as_bp_test_projectile (`self.As BP Test Projectile`))
  (return (+ Velocity (* (* (* (/ (`self.DragForce` (`self.Air Density`) (/ (`KismetMathLibrary.VSize` Velocity) 100.0) (`/Game/Blueprint/Weapon/Projectile/BP_Test_Projectile.BulletCrossSection` _as_bp_test_projectile) (`/Game/Blueprint/Weapon/Projectile/BP_Test_Projectile.Drag Coefficiency` _as_bp_test_projectile)) (`/Game/Blueprint/Weapon/Projectile/BP_Test_Projectile.BulletMass` _as_bp_test_projectile)) 100.0) (`KismetMathLibrary.Normal` (`local.Velocity`))) (`self.Delta Seconds`)) (`KismetMathLibrary.MakeVector` 0.0 0.0 (* (* (`self.Gravity`) -100.0) (`self.Delta Seconds`))))))

(fn `DragForce`
  (params (AirDensity :type "Float (double-precision)") (BulletSpeed :type "Float (double-precision)") (CrossSection :type "Float (double-precision)") (DragCoefficiency :type "Float (double-precision)"))
  (returns (DragForce :type "Float (double-precision)"))
  (return (* (/ (* (* (* AirDensity (`KismetMathLibrary.Square` BulletSpeed)) CrossSection) DragCoefficiency) 2.0) -1.0)))