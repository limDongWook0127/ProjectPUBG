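; Gameplay ability, named for an X press, that toggles between holstering the current weapon and drawing the last one.
; It plays montages by weapon type, slot and prone state, reversing them to equip guns.
; Montage events move the weapon between hand and back and add or remove its anim layer, input mapping, granted abilities and tag.
; Melee and throwable equip branches only play montages, without attaching or ending the ability.
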(event `SetAnimLayer`
  (params (InClass :type "AnimInstance Class Reference"))
  ;[1 1 1] 코멘트
  (`SkeletalMeshComponent.LinkAnimClassLayers` (`self.GetOwningComponentFromActorInfo`) InClass))

(event `RemoveWeaponAbility`
  (params (Target :type "Weapon_Base Object Reference"))
  ;[1 1 1] 코멘트
  (`BaseAbilitySystemComponent.RemoveGrantedPlayerWeaponAbilities` (`self.GetBaseAbilitySystemComponentFromActorInfo`) (`Weapon_Base.GetGrantedAbilitySpecHandles` Target)))

(event `SetWeaponAbility`
  (params (WeaponAbilities :type "Array of PlayerAbilitySet Structure (by ref)") (Target :type "Weapon_Base Object Reference"))
  ;[1 1 1] 코멘트
  (bind _outgrantedabilityspechandles (`BaseAbilitySystemComponent.GrantPlayerWeaponAbilities` (`self.GetBaseAbilitySystemComponentFromActorInfo`) WeaponAbilities (`self.GetAbilityLevel`)))
  (`Weapon_Base.AssignGrantedAbilitySpecHandles` Target _outgrantedabilityspechandles)
  (`KismetSystemLibrary.PrintString` "Hello"))

(event `self.K2_OnEndAbility`
  (params (bWasCancelled :type Boolean))
  (`BaseFunctionLibrary.RemoveGameplayTagFromActor` (`self.GetPlayerCharacterFromActorInfo`) (struct :`TagName` "Player.Ability.Weapon.Equip") true))

(event `self.K2_ActivateAbility`
  (bind _returnvalue (`self.GetPlayerCharacterFromActorInfo`))
  (`BaseFunctionLibrary.AddGameplayTagToActor` _returnvalue (struct :`TagName` "Player.Ability.Weapon.Equip") true)
  (`self.SetCanBeCanceled` false)
  (if (`KismetSystemLibrary.IsValid` (`EquippedComponent.GetLastCurrentWeapon` (`PlayerCharacter.EquippedComponent` _returnvalue)))
    (if (`self.IsValidCurrentWeapon`)
      (`self.PlayUnEquipMontage`)
      (else
        (`self.PlayerEquipMontage`)))
    (else
      (`self.K2_EndAbility`))))

(fn `EquipWeaponHandle`
  (params (self5 :type "Weapon_Base Object Reference"))
  (locals (NewLocalVar :type "PlayerAnimInstance Class Reference") (NewLocalVar_0 :type "PlayerAnimInstance Class Reference"))
  (bind (_weaponanimlayertolink _equipanimmontage _weapontag _weaponinputmappingcontext _weaponabilities) (break `PlayerWeaponData` (`Weapon_Base.PlayerWeaponData` self5)))
  (`/Engine/EditorBlueprintResources/StandardMacros.IsValid` self5
    (:`Is Valid`
      (`|ExecutionSequence`
        (:`then_0`
          (`PlayerCharacter.Server_SetAnimLayer` (`self.GetPlayerCharacterFromActorInfo`) _weaponanimlayertolink))
        (:`then_1`
          (`self.IsLocallyControlled`
            (:`True`
              (`EnhancedInputSubsystemInterface.AddMappingContext` (pcsubsystem `EnhancedInputLocalPlayerSubsystem` (`self.GetPlayerControllerFromActorInfo`)) _weaponinputmappingcontext 1 (struct)))))
        (:`then_2`
          (`self.SetWeaponAbility` _weaponabilities self5))
        (:`then_3`
          (`BaseFunctionLibrary.AddGameplayTagToActor` (`self.GetPlayerCharacterFromActorInfo`) _weapontag true))))
    (:`Is Not Valid`
      (`KismetSystemLibrary.PrintString` "No value"))))

(fn `UnEquipWeaponHandle`
  (params (Weapon :type "Weapon_Base Object Reference"))
  (bind (_weaponanimlayertolink _equipanimmontage _weapontag _weaponinputmappingcontext) (break `PlayerWeaponData` (`Weapon_Base.PlayerWeaponData` Weapon)))
  (`/Engine/EditorBlueprintResources/StandardMacros.IsValid` Weapon
    (:`Is Valid`
      (`|ExecutionSequence`
        (:`then_0`
          (`PlayerCharacter.Server_SetAnimLayer` (`self.GetPlayerCharacterFromActorInfo`) null))
        (:`then_1`
          (`self.IsLocallyControlled`
            (:`True`
              (`EnhancedInputSubsystemInterface.RemoveMappingContext` (pcsubsystem `EnhancedInputLocalPlayerSubsystem` (`self.GetPlayerControllerFromActorInfo`)) _weaponinputmappingcontext (struct)))))
        (:`then_2`
          (`self.RemoveWeaponAbility` Weapon))
        (:`then_3`
          (`BaseFunctionLibrary.RemoveGameplayTagFromActor` (`self.GetPlayerCharacterFromActorInfo`) _weapontag true))))
    (:`Is Not Valid`
      (`KismetSystemLibrary.PrintString` "No value"))))