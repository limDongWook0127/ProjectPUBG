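; GA_Hit is a Gameplay Ability that handles a weapon hit, playing feedback sounds and applying damage to the target.
; It activates from a gameplay event that supplies instigator, target and damage magnitude.
; HitSound plays a female pain voice tiered by damage, plus a random sound from the Sound array, at the target's location.
; ApplyDamageToActor then applies GE_Damage with that magnitude, and the ability ends on completion.
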(event `HitSound`
  (params (Location :type "Vector Structure") (Damage :type "Float (double-precision)"))
  (`|ExecutionSequence`
    (:`then_0`
      (`GameplayStatics.PlaySoundAtLocation` (select `bool` (> Damage 80.0) :`false` (select `bool` (> Damage 40.0) :`false` "/Game/PUBGAsset/Sounds/SFX/Voice_NoScript/_Female_Temp/Voice_Female_Damage_Weak_Temp_08_wem_Cue.Voice_Female_Damage_Weak_Temp_08_wem_Cue" :`true` "/Game/PUBGAsset/Sounds/SFX/Voice_NoScript/_Female_Temp/Voice_Female_Damage_Medium_Temp_01_wem_Cue.Voice_Female_Damage_Medium_Temp_01_wem_Cue" :!type "SoundBase Object Reference") :`true` "/Game/PUBGAsset/Sounds/SFX/Voice_NoScript/_Female_Temp/Voice_Female_Damage_Strong_Temp_02_wem_Cue.Voice_Female_Damage_Strong_Temp_02_wem_Cue") Location (struct) 1.0 1.0 0.0 "/Game/Blueprint/Map/MapSound/DoorSound.DoorSound" null null null))
    (:`then_1`
      (`GameplayStatics.PlaySoundAtLocation` (`KismetArrayLibrary.Array_Random` (`self.Sound`)) Location (struct) 1.0 1.0 0.0 null null null null))))

(event `self.K2_ActivateAbilityFromEvent`
  (params (EventData :type "GameplayEventData Structure (by ref)"))
  (bind (_eventtag _instigator _target _optionalobject _optionalobject2 _contexthandle _instigatortags _targettags _eventmagnitude) (break `GameplayEventData` EventData))
  (`self.HitSound` (`Actor.K2_GetActorLocation` _target) _eventmagnitude)
  (`ApplyDamageToActor.ApplyDamageToActor` null "None" _instigator _target "/Game/Blueprint/Character/GE/GE_Damage.GE_Damage_C" _eventmagnitude
    (:`OnCompleted`
      (`self.K2_EndAbility`))))