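; Gameplay ability that fires the sniper rifle, ending at once if the gun has no ammo.
; SpawnBullet plays a stance-based recoil montage and, only without authority, spawns a projectile from weapon data and applies recoil.
; After a short delay a follow-up montage plays, bracketed by CheckZoomIn and CheckZoomOut when zoomed.
; On end, an empty magazine triggers auto-reload through an ability tag.
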(event `self.K2_ActivateAbility`
  (bind _montage_to_play_0 (`self.Montage to Play_0`))
  (`self.SetCanBeCanceled` false)
  (if (> (`Gun_Base.GetBulletArmo` (`EquippedComponent.GetCurrentWeapon_GunBase` (`PlayerCharacter.EquippedComponent` (`self.GetPlayerCharacterFromActorInfo`)))) 0.0)
    (`self.SpawnBullet`
      (:`Success`
        (if (`PlayerCharacter.IsZoom` (`self.GetPlayerCharacterFromActorInfo`))
          ;[1 1 1] 단발
          (`self.CheckZoomIn`)
          (`KismetSystemLibrary.Delay` 0.2)
          (`PlayMontageAndWaitForEvent.PlayMontageAndWaitForEvent` "None" _montage_to_play_0 (struct) 2.0 "Default"
            (:`OnCompleted`
              _)
            (:`OnBlendOut`
              (`self.CheckZoomOut`))
            (:`OnInterrupted`
              _)
            (:`OnCancelled`
              _))
          (`self.K2_EndAbility`)
          (else
            (`KismetSystemLibrary.Delay` 0.2)
            (`PlayMontageAndWaitForEvent.PlayMontageAndWaitForEvent` "None" _montage_to_play_0 (struct) 2.0 "Default"
              (:`OnCompleted`
                _)
              (:`OnBlendOut`
                _)
              (:`OnInterrupted`
                _)
              (:`OnCancelled`
                _))
            (`self.K2_EndAbility`)))))
    (else
      (`self.K2_EndAbility`))))

(event `self.K2_OnEndAbility`
  (params (bWasCancelled :type Boolean))
  ;[1 1 1] 자동 재장전
  (if (<= (`Gun_Base.GetBulletArmo` (`EquippedComponent.GetCurrentWeapon_GunBase` (`PlayerCharacter.EquippedComponent` (`self.GetPlayerCharacterFromActorInfo`)))) 0.0)
    (`AbilitySystemComponent.TryActivateAbilitiesByTag` (`self.GetAbilitySystemComponentFromActorInfo`) (`self.Gameplay Tag Container`) true)))