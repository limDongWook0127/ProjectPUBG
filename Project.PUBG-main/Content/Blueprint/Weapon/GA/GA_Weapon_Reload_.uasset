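; Gameplay ability that reloads the player's equipped gun after an ammo check, and cannot be canceled.
; It checks zoom on non-authority instances and plays a montage chosen by prone reload state and whether the gun is empty.
; Montage gameplay events move the magazine between hand and gun and toggle its visibility, with the server recalculating ammo when it reappears.
; When the montage ends or is interrupted, the ability ends and refreshes HUD ammo from inventory and gun.
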(event `self.K2_ActivateAbility`
  (bind _reload_charge_true_montage (`self.Reload Charge True Montage`))
  (bind _returnvalue (`EquippedComponent.GetCurrentWeapon_GunBase` (`PlayerCharacter.EquippedComponent` (`self.GetPlayerCharacterFromActorInfo`))))
  (bind _returnvalue_2 (`EquippedComponent.GetCurrentWeapon_GunBase` (`PlayerCharacter.EquippedComponent` (`self.GetPlayerCharacterFromActorInfo`))))
  (bind _returnvalue_3 (`EquippedComponent.GetCurrentWeapon_GunBase` (`PlayerCharacter.EquippedComponent` (`self.GetPlayerCharacterFromActorInfo`))))
  (bind _returnvalue_4 (`Gun_Base.GetMagToHandSocekt` (`EquippedComponent.GetCurrentWeapon_GunBase` (`PlayerCharacter.EquippedComponent` (`self.GetPlayerCharacterFromActorInfo`)))))
  (bind _returnvalue_5 (`Gun_Base.GetMagToHandSocekt` (`EquippedComponent.GetCurrentWeapon_GunBase` (`PlayerCharacter.EquippedComponent` (`self.GetPlayerCharacterFromActorInfo`)))))
  (bind _returnvalue_6 (`Gun_Base.GetchangeValue` _returnvalue))
  (bind (_type _gunname _bullettype _gun_damage _armo) (break `WeaponData` (`Weapon_Base.GetWeaponDataAsset` _returnvalue)))
  (bind (_type_2 _gunname_2 _bullettype_2 _gun_damage_2 _armo_2) (break `WeaponData` (`Weapon_Base.GetWeaponDataAsset` _returnvalue_2)))
  (`self.SetCanBeCanceled` false)
  (`|ExecutionSequence`
    (:`then_0`
      (`self.K2_HasAuthority`
        (:`False`
          (`self.CheckZoom`))))
    (:`then_1`
      (if (`self.CheckCurrentBullet` _returnvalue_2 _armo_2 (`|GetEnumeratorName` _bullettype_2))
        (bind (_asynctaskproxy _eventtag) (`PlayMontageAndWaitForEvent.PlayMontageAndWaitForEvent` "None" (`self.selectCurrentMontage_isProne_Reload` (`|GetArrayItem` _reload_charge_true_montage) (`|GetArrayItem` _reload_charge_true_montage 1) (`|GetArrayItem` _reload_charge_true_montage 2) (`|GetArrayItem` _reload_charge_true_montage 3) (== (`Gun_Base.GetBulletArmo` _returnvalue_2) 0.0)) (struct :`GameplayTags` (struct :`(TagName` "Player.Event.Action.ReloadEnd") :`(TagName` "Player.Event.Action.Reload") :`(TagName` "Player.Event.Action.VisibleMag") :`(TagName` "Player.Event.Action.HideMag"))))
          (:`OnCompleted`
            (`self.K2_EndAbility` :!label _label)
            (`self.UpdateAmmoUIUpdate`))
          (:`OnBlendOut`
            (goto _label))
          (:`OnInterrupted`
            (goto _label))
          (:`OnCancelled`
            (goto _label))
          (:`EventReceived`
            (`|SwitchGameplayTag` _eventtag
              (:`Player.Event.Action.Reload`
                (`ActorComponent.SetIsReplicated` _returnvalue_5 true)
                (`SceneComponent.K2_AttachToComponent` _returnvalue_5 (`self.GetOwningComponentFromActorInfo`) "item_lSocket" "SnapToTarget" "SnapToTarget" "KeepRelative" true))
              (:`Player.Event.Action.ReloadEnd`
                (`SceneComponent.K2_AttachToComponent` (`Gun_Base.GetMagToHandSocekt` _returnvalue_3) (`Weapon_Base.WeaponSkeletalMeshComponent` _returnvalue_3) "MagSocket" "SnapToTarget" "SnapToTarget" "KeepRelative" true))
              (:`Player.Event.Action.HideMag`
                (`SceneComponent.SetVisibility` _returnvalue_4 false false))
              (:`Player.Event.Action.VisibleMag`
                (`SceneComponent.SetVisibility` _returnvalue_4 true false)
                (`self.K2_HasAuthority`
                  (:`True`
                    (`KismetSystemLibrary.PrintString` (`KismetStringLibrary.Conv_DoubleToString` _returnvalue_6))
                    (`self.SetReloadBullet_CalulateBullet` _returnvalue _armo _returnvalue_6 (`|GetEnumeratorName` _bullettype))))))))
        (else
          (`self.K2_EndAbility`))))))

(fn `UpdateAmmoUIUpdate`
  (bind _returnvalue (`self.GetPlayerCharacterFromActorInfo`))
  (bind _inventorycomponent (`PlayerCharacter.InventoryComponent` _returnvalue))
  (bind _returnvalue_2 (`EquippedComponent.GetCurrentWeapon_GunBase` (`PlayerCharacter.EquippedComponent` _returnvalue)))
  (bind _returnvalue_3 (`self.CheckBulletTypeName` (`|GetEnumeratorName` (`.BulletType` (break `WeaponData` (`Weapon_Base.GetWeaponDataAsset` _returnvalue_2))))))
  (bind _returnvalue_4 (`InventoryComponent.FindItemSlot` _inventorycomponent _returnvalue_3))
  (if (!= _returnvalue_4 -1)
    (bind _returnvalue_5 (`BasePlayerController.GetHudWidget` (`self.GetPlayerControllerFromActorInfo`)))
    (bind _returnvalue_6 (`KismetSystemLibrary.IsValid` _returnvalue_5))
    (if _returnvalue_6
      (bind _wbp_playerstatus (`HudWidget.WBP_PlayerStatus` _returnvalue_5))
      (`PlayerStatusWidget.SetText_Ammo` _wbp_playerstatus (`.Quantity` (break `ItemSlotStruct` (`|GetArrayItem` (`InventoryComponent.Content` _inventorycomponent) _returnvalue_4))))
      (`PlayerStatusWidget.SetText_CurrentAmmo` _wbp_playerstatus (`KismetMathLibrary.FTrunc` (`Gun_Base.GetBulletArmo` _returnvalue_2))))
    (elif _returnvalue_6
      (`PlayerStatusWidget.SetText_Ammo` (`HudWidget.WBP_PlayerStatus` _returnvalue_5) 0))))