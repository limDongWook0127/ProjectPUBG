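; Gameplay ability that reloads a shotgun ("SG"), starting only if a bullet check passes and refusing cancellation.
; It plays a charge montage whose gameplay events drive, on authority, looping reload, reload end and max-bullet checks.
; Without authority, those events refresh the HUD ammo, showing the gun's current rounds and the matching inventory quantity.
; The ability ends when the montage finishes, blends out or is interrupted, refreshing the HUD again.
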(event `self.K2_ActivateAbility`
  (bind _returnvalue (`EquippedComponent.GetCurrentWeapon_GunBase` (`PlayerCharacter.EquippedComponent` (`self.GetPlayerCharacterFromActorInfo`))))
  (bind _returnvalue_2 (`EquippedComponent.GetCurrentWeapon_GunBase` (`PlayerCharacter.EquippedComponent` (`self.GetPlayerCharacterFromActorInfo`))))
  (bind ((`BulletType` _bullettype) (`Armo` _armo)) (break `WeaponData` (`Gun_Base.GetWeaponDataAsset` _returnvalue)))
  (bind ((`BulletType` _bullettype_2) (`Armo` _armo_2)) (break `WeaponData` (`Weapon_Base.GetWeaponDataAsset` _returnvalue_2)))
  (bind _returnvalue_3 (`|GetEnumeratorName` _bullettype))
  (`self.SetCanBeCanceled` false)
  (if (`self.CheckBullet_SG` _returnvalue_2 _armo_2 (`|GetEnumeratorName` _bullettype_2))
    (bind (_asynctaskproxy _eventtag) (`PlayMontageAndWaitForEvent.PlayMontageAndWaitForEvent` "None" (`self.ChargeMontage`) (struct :`GameplayTags` (struct :`(TagName` "Player.Event.Action.ReloadEnd") :`(TagName` "Player.Event.Action.Reload") :`(TagName` "Player.Event.Action.VisibleMag") :`(TagName` "Player.Event.Action.HideMag"))) 1.0 "start")
      (:`OnCompleted`
        (`self.K2_EndAbility` :!label _label))
      (:`OnBlendOut`
        (goto _label))
      (:`OnInterrupted`
        (goto _label))
      (:`OnCancelled`
        (goto _label))
      (:`EventReceived`
        (`self.K2_HasAuthority`
          (:`True`
            (`|SwitchGameplayTag` _eventtag
              (:`Player.Event.Action.Reload`
                (`self.ReloadLooping` _returnvalue _returnvalue_3))
              (:`Player.Event.Action.ReloadEnd`
                (`self.ReloadEnd` _returnvalue _returnvalue_3))
              (:`Player.Event.Action.HideMag`
                (`self.CheckMaxReloadBullet` _returnvalue _armo))))
          (:`False`
            (`self.UpdateAmmoUIUpdate`)))))
    (else
      (`self.K2_EndAbility`))))

(event `UIUpdate`
  (`self.UpdateAmmoUIUpdate`))

(event `self.K2_OnEndAbility`
  (params (bWasCancelled :type Boolean))
  (`self.UpdateAmmoUIUpdate`))

(fn `UpdateAmmoUIUpdate`
  (bind _inventorycomponent (`PlayerCharacter.InventoryComponent` (`self.GetPlayerCharacterFromActorInfo`)))
  (bind _returnvalue (`EquippedComponent.GetCurrentWeapon_GunBase` (`PlayerCharacter.EquippedComponent` (`self.GetPlayerCharacterFromActorInfo`))))
  (bind _returnvalue_2 (`self.CheckBulletTypeName` (`|GetEnumeratorName` (`.BulletType` (break `WeaponData` (`Weapon_Base.GetWeaponDataAsset` _returnvalue))))))
  (bind _returnvalue_3 (`InventoryComponent.FindItemSlot` _inventorycomponent _returnvalue_2))
  (if (!= _returnvalue_3 -1)
    (bind _returnvalue_4 (`BasePlayerController.GetHudWidget` (`self.GetPlayerControllerFromActorInfo`)))
    (bind _returnvalue_5 (`KismetSystemLibrary.IsValid` _returnvalue_4))
    (if _returnvalue_5
      (bind _wbp_playerstatus (`HudWidget.WBP_PlayerStatus` _returnvalue_4))
      (`PlayerStatusWidget.SetText_Ammo` _wbp_playerstatus (`.Quantity` (break `ItemSlotStruct` (`|GetArrayItem` (`InventoryComponent.Content` _inventorycomponent) _returnvalue_3))))
      (`PlayerStatusWidget.SetText_CurrentAmmo` _wbp_playerstatus (`KismetMathLibrary.FTrunc` (`Gun_Base.GetBulletArmo` _returnvalue))))
    (elif _returnvalue_5
      (`PlayerStatusWidget.SetText_Ammo` (`HudWidget.WBP_PlayerStatus` _returnvalue_4) 0))))