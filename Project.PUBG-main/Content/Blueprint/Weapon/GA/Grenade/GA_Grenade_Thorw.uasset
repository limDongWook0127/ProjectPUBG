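; Gameplay ability for throwing a grenade, with montages chosen for prone or standing.
; Activation plays the wind-up montage and adds a replicated ThrowsReady tag.
; Ending starts the throw montage, which outlives the ability, and immediately clears that tag.
; It then strips the current weapon's granted abilities, local input mapping context and weapon tag, and calls the server to set the anim layer.
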(event `RemoveAbility`
  (params (`타깃` :type "Weapon_Base Object Reference"))
  ;[1 1 1] 코멘트
  (`BaseAbilitySystemComponent.RemoveGrantedPlayerWeaponAbilities` (`self.GetBaseAbilitySystemComponentFromActorInfo`) (`Weapon_Base.GetGrantedAbilitySpecHandles` `타깃`)))

(event `self.K2_ActivateAbility`
  (`PlayMontageAndWaitForEvent.PlayMontageAndWaitForEvent` "None" (`self.selectCurrentMontage_isProne_Throw` "/Game/Blueprint/Character/Animation/AnimAssets/Weapon/Grenade/Throw/ThrowPose_F_BaseBody_01_Grenade_Combat_Prone_Start_Montage.ThrowPose_F_BaseBody_01_Grenade_Combat_Prone_Start_Montage" "/Game/Blueprint/Character/Animation/AnimAssets/Weapon/Grenade/Throw/ThrowPose_F_BaseBody_01_Grenade_Combat_Stand_Start_Montage.ThrowPose_F_BaseBody_01_Grenade_Combat_Stand_Start_Montage") (struct) 2.0
    (:`then`
      (`BaseFunctionLibrary.AddGameplayTagToActor` (`self.GetPlayerCharacterFromActorInfo`) (struct :`TagName` "Player.State.ThrowsReady") true))))

(event `self.K2_OnEndAbility`
  (params (bWasCancelled :type Boolean))
  (`PlayMontageAndWaitForEvent.PlayMontageAndWaitForEvent` "None" (`self.selectCurrentMontage_isProne_Throw` "/Game/Blueprint/Character/Animation/AnimAssets/Weapon/Grenade/Throw/ThrowPose_F_BaseBody_01_Grenade_Combat_Prone_High_End_Montage.ThrowPose_F_BaseBody_01_Grenade_Combat_Prone_High_End_Montage" "/Game/Blueprint/Character/Animation/AnimAssets/Weapon/Grenade/Throw/ThrowPose_F_BaseBody_01_Grenade_Combat_Stand_High_End_Montage.ThrowPose_F_BaseBody_01_Grenade_Combat_Stand_High_End_Montage") (struct :`GameplayTags` (struct :`(TagName` "Player.Event.Action.Throw"))) 2.0 "None" false
    (:`then`
      (`BaseFunctionLibrary.RemoveGameplayTagFromActor` (`self.GetPlayerCharacterFromActorInfo`) (struct :`TagName` "Player.State.ThrowsReady") true)
      (`self.Remove` (`EquippedComponent.GetCurrentWeapon` (`PlayerCharacter.EquippedComponent` (`self.GetPlayerCharacterFromActorInfo`)))))))

(fn `Remove`
  (params (`타깃` :type "Weapon_Base Object Reference"))
  (bind (_weaponanimlayertolink _equipanimmontage _weapontag _weaponinputmappingcontext) (break `PlayerWeaponData` (`Weapon_Base.PlayerWeaponData` `타깃`)))
  (`/Engine/EditorBlueprintResources/StandardMacros.IsValid` `타깃`
    (:`Is Valid`
      (`|ExecutionSequence`
        (:`then_0`
          (`PlayerCharacter.Server_SetAnimLayer` (`self.GetPlayerCharacterFromActorInfo`) null))
        (:`then_1`
          (`self.IsLocallyControlled`
            (:`True`
              (`EnhancedInputSubsystemInterface.RemoveMappingContext` (pcsubsystem `EnhancedInputLocalPlayerSubsystem` (`self.GetPlayerControllerFromActorInfo`)) _weaponinputmappingcontext (struct)))))
        (:`then_2`
          (`self.RemoveAbility` `타깃`))
        (:`then_3`
          (`BaseFunctionLibrary.RemoveGameplayTagFromActor` (`self.GetPlayerCharacterFromActorInfo`) _weapontag true))))
    (:`Is Not Valid`
      (`KismetSystemLibrary.PrintString` "No value"))))