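; Base gun Blueprint that loads its weapon data from a data table.
; On BeginPlay, Setting looks up the row named by WeaponDataTableRowName in DT_WeaponData and passes it to SetWeaponDataAsset.
; When the row is found, it also prints whether it runs on server or client and resizes the WeaponParts array to a fixed slot count.
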(event `self.ReceiveBeginPlay`
  (`self.Setting`))

(fn `Setting`
  ;[1 1 1] Comment
  (bind _returnvalue (`|GetDataTableRow` "/Game/Blueprint/Weapon/Datatable/DT_WeaponData.DT_WeaponData" (`self.WeaponDataTableRowName`))
    (:`then`
      (`self.SetWeaponDataAsset` _returnvalue)
      (if (`self.HasAuthority`)
        (`KismetSystemLibrary.PrintString` "Server")
        (else
          (`KismetSystemLibrary.PrintString` "Client")))
      (`KismetArrayLibrary.Array_Resize` (`self.WeaponParts`) 5))))

(fn `UserConstructionScript`)