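; Throwable grenade weapon Blueprint that loads its weapon data from DT_WeaponData on BeginPlay.
; Throw launches it through ProjectileMovement at a scaled velocity and calls SettingThrowable after a short delay.
; A parallel fixed fuse delay spawns a pooled Niagara explosion at the mesh location, then activates hit collision just after the effect starts.
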(event `self.ReceiveBeginPlay`
  (bind _returnvalue (`|GetDataTableRow` "/Game/Blueprint/Weapon/Datatable/DT_WeaponData.DT_WeaponData" (`self.WeaponDataTableRowName`))
    (:`then`
      (`self.SetWeaponDataAsset` _returnvalue))))

(event `Throw`
  (params (`속도` :type "Vector Structure"))
  (bind _projectilemovement (`self.ProjectileMovement`))
  (`|ExecutionSequence`
    (:`then_0`
      (`ActorComponent.Activate` _projectilemovement false)
      (set `MovementComponent.Velocity` (* `속도` 2000.0) _projectilemovement))
    (:`then_1`
      (`KismetSystemLibrary.Delay` 7.0)
      (`NiagaraFunctionLibrary.SpawnSystemAtLocation` "/Game/PUBGAsset/Weapon_Assets/VFX/Expose/MsvFx_Niagara_Explosion_Pack_01/Prefabs/Niagara_Explosion_03.Niagara_Explosion_03" (.location (`SceneComponent.K2_GetComponentToWorld` (`self.WeaponSkeletalMeshComponent`))) (struct :`Pitch` 90.0) (.scale (`SceneComponent.K2_GetComponentToWorld` (`self.WeaponSkeletalMeshComponent`))) true true "AutoRelease")
      (`KismetSystemLibrary.Delay` 0.15)
      (`self.SetHitCollisionActivate`))
    (:`then_2`
      (`KismetSystemLibrary.Delay` 1.0)
      (`self.SettingThrowable`))))

(fn `UserConstructionScript`)